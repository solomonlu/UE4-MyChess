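; Chessboard actor that spawns a BP_ChessPosition actor for each of the 64 squares of an 8x8 board.
; The construction script derives cell size and the corner square's offset from the SMChessPanel mesh bounds.
; On BeginPlay, a loop converts each index to a column and row offset, transforms it by the actor's transform and passes the index to the spawned square.
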(event `self.ReceiveBeginPlay`
  (bind (_cellsize_x _cellsize_y) (`KismetMathLibrary.BreakVector2D` (`self.CellSize`)))
  (for _index (range 64)
    (`|SpawnActorFromClass` "/Game/MyChess/Blueprints/BP_ChessPosition.BP_ChessPosition_C" (`KismetMathLibrary.MakeTransform` (`KismetMathLibrary.TransformLocation` (`self.GetTransform`) (+ (`KismetMathLibrary.MakeVector` (* (mod _index 8) _cellsize_x) (* (* (/ _index 8) _cellsize_y) -1.0)) (`self.LeftDownPositionOffset`)))) "Undefined" "OverrideRootScale" null _index)))

(fn `UserConstructionScript`
  (bind (_origin _boxextent) (`KismetSystemLibrary.GetComponentBounds` (`self.SM_ChessPanel`)))
  (bind _output_get (set `self.CellSize` (`KismetMathLibrary.MakeVector2D` (/ (.x _boxextent) 4.0) (/ (.y _boxextent) 4.0))))
  (set `self.LeftDownPositionOffset` (`KismetMathLibrary.MakeVector` (* (`KismetMathLibrary.BreakVector2D` _output_get) -3.5) (* (`.Y` (`KismetMathLibrary.BreakVector2D` _output_get)) 3.5))))