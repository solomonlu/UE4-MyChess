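; BP_PC_Game is the chess game's player controller, letting the player move pieces by clicking.
; On left-click release with nothing selected, a cursor trace against Pawns stores the hit BP_ChessmanBase as the selected piece.
; With a piece selected, a trace on a custom object type finds a BP_ChessPosition, moves the piece above it and clears the selection.
; The file contains no move validation or turn logic.
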(event `InputAction|LeftMouseClick`
  (params (Key :type "Key Structure" :default "AnyKey"))
  (:`Released`
    (`self.SelectedChessman`
      (:`then`
        (bind _asbp_chess_position (cast `/Game/MyChess/Blueprints/BP_ChessPosition` (`.HitActor` (`GameplayStatics.BreakHitResult` (`self.GetHitResultUnderCursorForObjects` (`|MakeArray` "ObjectTypeQuery7" :!type "EObjectTypeQuery Enum") false)))))
        (`self.K2_SetActorLocation` (`self.SelectedChessman`) (+ (`self.K2_GetActorLocation` _asbp_chess_position) (0.0 0.0 250.0)) false false)
        (set `self.SelectedChessman` null))
      (:`else`
        (bind _asbp_chessman_base (cast `/Game/MyChess/Blueprints/Chessman/BP_ChessmanBase` (`.HitActor` (`GameplayStatics.BreakHitResult` (`self.GetHitResultUnderCursorForObjects` (`|MakeArray` "ObjectTypeQuery3" :!type "EObjectTypeQuery Enum") false)))))
        (set `self.SelectedChessman` _asbp_chessman_base)))))

(fn `UserConstructionScript`)